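; Tiger_BP is the player tank Blueprint, wiring tank components together and handling camera aim input.
; On BeginPlay it passes barrel and turret references to the aiming component and track references to the movement component, with TracksRight assigned as LeftTrack and vice versa.
; It also sets the barrel reference on itself.
; Aim axis inputs yaw a horizontal gimbal and pitch the spring arm independently.
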(event `self.ReceiveBeginPlay`
  (bind _tankaimingcomponent (`self.TankAimingComponent`))
  (bind _tankbarrel (`self.TankBarrel`))
  (`self.SetBarrelReference` _tankbarrel)
  (`TankAimingComponent.SetBarrelReference` _tankaimingcomponent _tankbarrel)
  (`TankAimingComponent.SetTurretReference` _tankaimingcomponent (`self.TankTurret`))
  (`TankMovementComponent.SetTracksReference` (`self.TankMovementComponent`) (`self.TracksRight`) (`self.TracksLeft`)))

(event `InputAxis|AimHorizontal`
  (params (AxisValue :type "Float (single-precision)"))
  (`SceneComponent.K2_AddLocalRotation` (`self.HorizontalGimbal`) (`KismetMathLibrary.MakeRotator` 0.0 0.0 AxisValue) false false))

(event `InputAxis|AimVertical`
  (params (AxisValue :type "Float (single-precision)"))
  (`SceneComponent.K2_AddLocalRotation` (`self.SpringArm`) (`KismetMathLibrary.MakeRotator` 0.0 AxisValue) false false))

(fn `UserConstructionScript`)