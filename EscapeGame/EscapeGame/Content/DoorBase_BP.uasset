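; DoorBase_BP is a door actor that swings open and closed by rotating around its yaw axis.
; Open, chill and close request events from Door play, stop or reverse the DoorSwing timeline.
; On BeginPlay it caches the initial rotation and divides the timeline's play rate by the configured duration.
; The timeline's curve scales the configured angle on top of that rotation, and an event track plays the lock sound.
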(event `self.ReceiveBeginPlay`
  (set `self.Initial Rotation` (`self.K2_GetActorRotation`))
  (set `self.PlayRate` (/ (`TimelineComponent.GetPlayRate` (`self.Door Swing`)) (`Door.RotationDuration` (`self.Door`))))
  (`TimelineComponent.SetPlayRate` (`self.Door Swing`) (`self.PlayRate`))
  (bind (_direction _openangle) (`Timeline|Door Swing` :!via `SetNewTime` :!label _label)
    (:`Update`
      (`self.K2_SetActorRotation` (`KismetMathLibrary.ComposeRotators` (`KismetMathLibrary.MakeRotator` 0.0 0.0 (* (`Door.RotationAngle` (`self.Door`)) _openangle)) (`self.Initial Rotation`))))
    (:`Sound Timing`
      (`GameplayStatics.PlaySoundAtLocation` "/Game/Audio/door-lock.door-lock" (`self.K2_GetActorLocation`)))))

(event `self.Door.OpenRequest`
  (goto _label))

(event `self.Door.ChillRequest`
  (goto _label :!via `Stop`))

(event `self.Door.CloseRequest`
  (goto _label :!via `Reverse`))

(fn `UserConstructionScript`)